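; Base pickup actor for a TPS game, carrying a shape type and a score in its PickupData.
; On construction, Init selects a primitive mesh by type and prints the score on a TextRender.
; A random ColorPalette color tints both the text and a dynamic material instance on the mesh, so it can change whenever construction reruns.
; EndPlay spawns a Niagara explosion at the actor's location, whatever the reason play ends.
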(event EventEndPlay
  (params (EndPlayReason :type EEndPlayReason%20Enum :default "Destroyed"))
  (Niagara|SpawnSystematLocation "/Game/FX/NS_Explosition.NS_Explosition" (Transformation|GetActorLocation)))

(fn ConstructionScript
  (CallFunction|Init))

(fn Init
  (Components|StaticMesh|SetStaticMesh (Variables|Default|GetStaticMesh) (Utilities|Select :Index (.Type (Utilities|Struct|BreakPickupData (Variables|Default|GetPickupData))) :EPT_SPHERE "/Engine/BasicShapes/Sphere.Sphere" :EPT_CUBE "/Game/LevelPrototyping/Meshes/SM_ChamferCube.SM_ChamferCube" :EPT_CYLINDER "/Engine/BasicShapes/Cylinder.Cylinder" :EPT_CONE "/Engine/BasicShapes/Cone.Cone"))
  (LocalVariables|SetItemColor (CallFunction|GenerateColor))
  (Rendering|Components|TextRender|SetTextRenderColor (Variables|Default|GetTextRender) (Math|Conversions|ToColor(LinearColor) (LocalVariables|GetItemColor)))
  (bind _returnvalue (Rendering|Material|CreateDynamicMaterialInstance (Variables|Default|GetStaticMesh) 0 "/Game/Materials/Instances/MI_BaseColor.MI_BaseColor" "None" :!class /Script/Engine.PrimitiveComponent))
  (Rendering|Material|SetVectorParameterValue _returnvalue "BaseColor" (LocalVariables|GetItemColor) :!class /Script/Engine.MaterialInstanceDynamic)
  (Rendering|Components|TextRender|SetText (Variables|Default|GetTextRender) (Utilities|Text|ToText(Integer) (.Score (Utilities|Struct|BreakPickupData (Variables|Default|GetPickupData))))))

(fn GenerateColor
  (return (.OutItem (Utilities|Array|Random (Variables|Default|GetColor%20Palette)))))