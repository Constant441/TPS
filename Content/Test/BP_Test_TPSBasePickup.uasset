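; BP_Test_TPSBasePickup is a test pickup Blueprint that allows its data and color to be set from outside.
; SetPickupData stores the supplied PickupData and color, then calls Init.
; GenerateColor returns the stored TestColor, so the pickup's color is controlled by the caller.
; BeginPlay, overlap, Tick and the construction script only forward to the parent class.
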(event Custom|SetPickupData
  (params (PickupData :type Pickup%20Data%20Structure) (Color :type Linear%20Color%20Structure))
  (Variables|Default|SetPickupData PickupData)
  (Variables|Default|SetTestColor Color)
  (CallFunction|Init))

(event EventBeginPlay
  (|CallParentFunction))

(event Collision|EventActorBeginOverlap
  (params (OtherActor :type Actor%20Object%20Reference))
  (|CallParentFunction OtherActor))

(event EventTick
  (params (DeltaSeconds :type Float%20%28single-precision%29))
  (|CallParentFunction DeltaSeconds))

(fn ConstructionScript
  (|CallParentFunction))

(fn GenerateColor
  (return (Variables|Default|GetTestColor)))